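; BP_TestPawn is a player pawn that moves in grid steps through the die world on a limited step budget.
; WASD presses line-trace for blockers, then subtract a step from BP_DieDefinition and teleport by its step size, with DoOnce gating each press.
; Tick resets the step budget, key count and level through BP_LevelMapManager when steps drop below zero.
; M pitches the die actor 90 degrees.
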(event EventBeginPlay
  (bind _returnvalue (Actor|GetActorOfClass "/Game/Blueprints/DieWorld/BP_DieDefinition.BP_DieDefinition_C"))
  (Variables|Default|SetWorldref _returnvalue)
  (bind _returnvalue_2 (Actor|GetActorOfClass "/Game/Blueprints/Objects/BP_LevelMapManager.BP_LevelMapManager_C"))
  (Variables|LevelManagement|SetLevelManagerRef _returnvalue_2)
  (Variables|Default|SetXStepSize (Variables|/Game/Blueprints/DieWorld/BP_DieDefinition.BP_DieDefinition_C|GetXStepSize (Variables|Default|GetWorldref)))
  (Variables|Default|SetYStepSize (Variables|/Game/Blueprints/DieWorld/BP_DieDefinition.BP_DieDefinition_C|GetYStepSize (Variables|Default|GetWorldref)))
  (Variables|Default|SetResetPosition (Transformation|GetActorLocation))
  (Variables|Default|SetAmountOfKeysCollected 0))

(event EventTick
  (params (DeltaSeconds :type Float%20%28single-precision%29))
  (if (< (Variables|/Game/Blueprints/DieWorld/BP_DieDefinition.BP_DieDefinition_C|GetAmountOfSteps (Variables|Default|GetWorldref)) 0)
    (CallFunction|ResetPlayer)))

(event Input|KeyboardEvents|M
  (params (Key :type Key%20Structure :default "None"))
  (bind _worldref (Variables|Default|GetWorldref))
  (bind _returnvalue (Transformation|GetActorRotation _worldref))
  (:Pressed
    (Utilities|FlowControl|DoOnce false :!label _label
      (:Completed
        (Transformation|SetActorRotation _worldref (Math|Rotator|MakeRotator (.roll _returnvalue) (+ (.pitch _returnvalue) 9e+01) (.yaw _returnvalue))))))
  (:Released
    (goto _label Reset)))

(event Input|KeyboardEvents|D
  (params (Key :type Key%20Structure :default "None"))
  (bind _returnvalue (Transformation|GetActorLocation))
  (bind _self self)
  (bind _returnvalue_2 (Transformation|GetActorLocation _self))
  (:Pressed
    ;[1 1 1] Checks collision
    (bind _returnvalue_3 (Collision|LineTraceByChannel (Transformation|GetActorLocation) (Math|Vector|MakeVector (+ (Variables|Default|GetXStepSize) (.x _returnvalue)) (.y _returnvalue) (.z _returnvalue)) "TraceTypeQuery1" false 0 "None"))
    (if (not _returnvalue_3)
      (Utilities|FlowControl|DoOnce false :!label _label
        (:Completed
          ;[1 1 1] Do a step
          (CallFunction|SubstractSteps 1)
          (if (not (< (Variables|/Game/Blueprints/DieWorld/BP_DieDefinition.BP_DieDefinition_C|GetAmountOfSteps (Variables|Default|GetWorldref)) 0))
            (Transformation|SetActorLocation (Math|Vector|MakeVector (+ (.x _returnvalue_2) (Variables|Default|GetXStepSize)) (.y _returnvalue_2) (.z _returnvalue_2)) false false))))))
  (:Released
    (goto _label Reset)))

(event Input|KeyboardEvents|A
  (params (Key :type Key%20Structure :default "None"))
  (bind _returnvalue (Transformation|GetActorLocation))
  (bind _self self)
  (bind _returnvalue_2 (Transformation|GetActorLocation _self))
  (:Pressed
    (bind _returnvalue_3 (Collision|LineTraceByChannel (Transformation|GetActorLocation) (Math|Vector|MakeVector (- (.x _returnvalue) (Variables|Default|GetXStepSize)) (.y _returnvalue) (.z _returnvalue)) "TraceTypeQuery1" false 0 "None"))
    (if (not _returnvalue_3)
      (Utilities|FlowControl|DoOnce false :!label _label
        (:Completed
          (CallFunction|SubstractSteps 1)
          (if (not (< (Variables|/Game/Blueprints/DieWorld/BP_DieDefinition.BP_DieDefinition_C|GetAmountOfSteps (Variables|Default|GetWorldref)) 0))
            (Transformation|SetActorLocation (Math|Vector|MakeVector (- (.x _returnvalue_2) (Variables|Default|GetXStepSize)) (.y _returnvalue_2) (.z _returnvalue_2)) false false))))))
  (:Released
    (goto _label Reset)))

(event Input|KeyboardEvents|W
  (params (Key :type Key%20Structure :default "None"))
  (bind _returnvalue (Transformation|GetActorLocation))
  (bind _self self)
  (bind _returnvalue_2 (Transformation|GetActorLocation _self))
  (:Pressed
    (bind _returnvalue_3 (Collision|LineTraceByChannel (Transformation|GetActorLocation) (Math|Vector|MakeVector (.x _returnvalue) (- (.y _returnvalue) (Variables|Default|GetYStepSize)) (.z _returnvalue)) "TraceTypeQuery1" false 0 "None"))
    (if (not _returnvalue_3)
      (Utilities|FlowControl|DoOnce false :!label _label
        (:Completed
          (if (not (< (Variables|/Game/Blueprints/DieWorld/BP_DieDefinition.BP_DieDefinition_C|GetAmountOfSteps (Variables|Default|GetWorldref)) 0))
            (CallFunction|SubstractSteps 1)
            (Transformation|SetActorLocation (Math|Vector|MakeVector (.x _returnvalue_2) (- (.y _returnvalue_2) (Variables|Default|GetYStepSize)) (.z _returnvalue_2)) false false))))))
  (:Released
    (goto _label Reset)))

(event Input|KeyboardEvents|S
  (params (Key :type Key%20Structure :default "None"))
  (bind _returnvalue (Transformation|GetActorLocation))
  (bind _self self)
  (bind _returnvalue_2 (Transformation|GetActorLocation _self))
  (:Pressed
    (bind _returnvalue_3 (Collision|LineTraceByChannel (Transformation|GetActorLocation) (Math|Vector|MakeVector (.x _returnvalue) (+ (Variables|Default|GetYStepSize) (.y _returnvalue)) (.z _returnvalue)) "TraceTypeQuery1" false 0 "None"))
    (if (not _returnvalue_3)
      (Utilities|FlowControl|DoOnce false :!label _label
        (:Completed
          (CallFunction|SubstractSteps 1)
          (if (not (< (Variables|/Game/Blueprints/DieWorld/BP_DieDefinition.BP_DieDefinition_C|GetAmountOfSteps (Variables|Default|GetWorldref)) 0))
            (Transformation|SetActorLocation (Math|Vector|MakeVector (.x _returnvalue_2) (+ (.y _returnvalue_2) (Variables|Default|GetYStepSize)) (.z _returnvalue_2)) false false))))))
  (:Released
    (goto _label Reset)))

(fn ConstructionScript)

(fn SubstractSteps
  (params (Amount :type Integer))
  (bind _worldref (Variables|Default|GetWorldref))
  (Variables|/Game/Blueprints/DieWorld/BP_DieDefinition.BP_DieDefinition_C|SetAmountOfSteps _worldref (- (Variables|/Game/Blueprints/DieWorld/BP_DieDefinition.BP_DieDefinition_C|GetAmountOfSteps _worldref) Amount)))

(fn ResetPlayer
  (bind _worldref (Variables|Default|GetWorldref))
  (Variables|/Game/Blueprints/DieWorld/BP_DieDefinition.BP_DieDefinition_C|SetAmountOfSteps _worldref (Variables|/Game/Blueprints/DieWorld/BP_DieDefinition.BP_DieDefinition_C|GetMaxStepsThisLevel _worldref))
  (Variables|Default|SetAmountOfKeysCollected 0)
  (Default|CallPlayerReset)
  (Default|ResetLevel (Variables|LevelManagement|GetLevelManagerRef)))