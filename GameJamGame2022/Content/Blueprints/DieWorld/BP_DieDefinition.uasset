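; BP_DieDefinition is the die actor that turns between levels and holds the step budget for the current one.
; StartRotating takes the next rotation from BP_LevelMapManager and has it unload the level, then Tick lerps the actor there over about a second.
; When the turn finishes, the manager loads the next level and the step count resets from its budget.
; Tick also prints the remaining steps every frame.
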(event EventBeginPlay
  (bind _returnvalue (Actor|GetActorOfClass "/Game/Blueprints/Objects/BP_LevelMapManager.BP_LevelMapManager_C"))
  (Variables|LevelManager|SetLevelManagerRef _returnvalue)
  (Utilities|FlowControl|Delay 0.0)
  (CallFunction|SetStepBudget))

(event Collision|EventActorBeginOverlap
  (params (OtherActor :type Actor%20Object%20Reference)))

(event EventTick
  (params (DeltaSeconds :type Float%20%28single-precision%29))
  (Development|PrintString (Utilities|String|ToString(Integer) (Variables|Default|GetAmountOfSteps)))
  (if (Variables|Rotation|GetIsRotating)
    (Variables|Rotation|SetRotationIntererpelation (+ (Variables|Rotation|GetRotationIntererpelation) DeltaSeconds))
    (Transformation|SetActorRotation (Math|Rotator|Lerp(Rotator) (Variables|Rotation|GetStartRotation) (Variables|Rotation|GetEndRotation) (Math|Float|Clamp(Float) (Variables|Rotation|GetRotationIntererpelation))))
    (if (> (Variables|Rotation|GetRotationIntererpelation) 1.0)
      (Variables|Rotation|SetIsRotating false)
      (Default|LoadNextLevel (Variables|LevelManager|GetLevelManagerRef))
      (CallFunction|SetStepBudget))))

(fn ConstructionScript)

(fn StartRotating
  (Variables|Rotation|SetIsRotating true)
  (Variables|Rotation|SetStartRotation (Transformation|GetActorRotation))
  (Variables|Rotation|SetEndRotation (Variables|/Game/Blueprints/Objects/BP_LevelMapManager.BP_LevelMapManager_C|GetNextDieRotation (Variables|LevelManager|GetLevelManagerRef)))
  (Variables|Rotation|SetRotationIntererpelation 0.0)
  (Default|UnloadLevel (Variables|LevelManager|GetLevelManagerRef)))

(fn SetStepBudget
  (bind _output_get (Variables|Default|SetMaxStepsThisLevel (Variables|/Game/Blueprints/Objects/BP_LevelMapManager.BP_LevelMapManager_C|GetCurrentStepBudget (Variables|LevelManager|GetLevelManagerRef))))
  (Variables|Default|SetAmountOfSteps _output_get))