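; Grid actor that builds a flat checkerboard of BP_GridCell actors on BeginPlay, sized by grid width, height and cell size.
; Each cell is spawned, scaled, attached to the grid, offset by its grid position and given an even or odd material from coordinate parity.
; Cells are stored row by row, so GetWorldPosition maps a grid coordinate to a cell's location, printing an error when out of bounds.
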(event Custom|SpawnTile
  (params (GridPosition :type Vector%202D%20Structure))
  (GridCreation|SpawnGridCell GridPosition))

(event EventBeginPlay
  (GridCreation|SpawnGrid))

(fn ConstructionScript)

(fn SpawnGrid
  (for _index (range 0 (- (Variables|Dimensions|GetGridHeight) 1))
    (for _index_2 (range 0 (- (Variables|Dimensions|GetGridWidth) 1))
      (CallFunction|SpawnTile (Math|Vector2D|MakeVector2D (Math|Conversions|ToFloat(Integer) _index_2) (Math|Conversions|ToFloat(Integer) _index))))))

(fn SpawnGridCell
  (params (GridPosition :type Vector%202D%20Structure))
  (bind _returnvalue (Game|SpawnActorfromClass "/Game/Blueprints/Grid/BP_GridCell.BP_GridCell_C" (Transformation|GetActorTransform) "Undefined" 0 0))
  (bind _output_get (LocalVariables|SetSpawnedGridCell _returnvalue))
  (Variables|/Game/Blueprints/Grid/BP_GridCell.BP_GridCell_C|SetGridPosition _output_get GridPosition)
  (Transformation|SetActorScale3D (LocalVariables|GetSpawnedGridCell) (Dimensions|GetCellScale))
  (Transformation|AttachActorToActor (LocalVariables|GetSpawnedGridCell) self "None" "KeepRelative" "KeepRelative" "KeepRelative" true)
  (Transformation|SetRelativeLocation (Variables|/Game/Blueprints/Grid/BP_GridCell.BP_GridCell_C|GetDefaultSceneRoot (LocalVariables|GetSpawnedGridCell)) (Dimensions|GetCellPosition GridPosition) false false)
  (GridCreation|SetCellMaterial (LocalVariables|GetSpawnedGridCell) GridPosition)
  (Utilities|Array|Add (Variables|Default|GetGridCells) (LocalVariables|GetSpawnedGridCell)))

(fn GetCellScale
  (bind _cellsize (Variables|Dimensions|GetCellSize))
  (return (Math|Vector|MakeVector (.x _cellsize) (.y _cellsize) 0.0)))

(fn GetCellPosition
  (params (PositionInGrid :type Vector%202D%20Structure))
  (bind _cellsize (Variables|Dimensions|GetCellSize))
  (bind _returnvalue (* PositionInGrid _cellsize))
  (return (Math|Vector|MakeVector (.x _returnvalue) (.y _returnvalue) 0.0)))

(fn GridPositionIsEven
  (params (GridPosition :type Vector%202D%20Structure))
  (return (== (Class|KismetMathLibrary|AndInt64Int64 (+ (.x GridPosition) (.y GridPosition)) 1) 0)))

(fn SetCellMaterial
  (params (GridCell :type BP%20Grid%20Cell%20Object%20Reference) (GridPosition :type Vector%202D%20Structure))
  (if (GridCreation|GridPositionIsEven GridPosition)
    (Default|SetColor GridCell (Variables|Materials|GetEvenMaterial))
    (else
      (Default|SetColor GridCell (Variables|Materials|GetOddMaterial)))))

(fn GetWorldPosition
  (params (GridPosition :type Vector%202D%20Structure))
  (if (Math|Boolean|ANDBoolean (< (.x GridPosition) (Variables|Dimensions|GetGridWidth)) (>= (.x GridPosition) 0.0) (< (.y GridPosition) (Variables|Dimensions|GetGridHeight)) (>= (.y GridPosition) 0.0))
    (return (Default|GetWorldPosition (Utilities|Array|Get(acopy) (Variables|Default|GetGridCells) (Math|Float|Truncate (+ (.x GridPosition) (* (.y GridPosition) (Variables|Dimensions|GetGridWidth)))))))
    (else
      (Development|PrintString "The Provided grid position does not exist" true true "(R=1.000000,G=0.000000,B=0.092549,A=1.000000)" 2e+01)
      (return "0, 0, 0"))))