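; Level manager that builds each grid level from a tilemap and handles level progression and resets.
; LoadNextLevel counts CurrentLevel down, signalling game cleared at zero, and LoadLevel looks up that level's tilemap in DT_LevelBudgets.
; SpawnObjects reads tile user data to spawn the possessed player, keys, hazards, directional enemies and exits, plus alternating-material floor indicators.
; Spawned actors are tracked in GridItems and GridTiles, which UnloadLevel destroys before reloading.
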(event Custom|LoadNextLevel
  ;[1 1 1] Unload the previous level and load the next level
  (bind _result (Math|Integer|DecrementInt (Variables|Default|GetCurrentLevel))
    (:%20%20
      (if (!= _result 0)
        (LevelUnloading|UnloadLevel)
        (LevelLoading|LoadLevel)
        (else
          (Default|CallGameCleared))))))

(event Custom|ResetLevel
  ;[1 1 1] Reset level
  (LevelUnloading|UnloadLevel)
  (LevelLoading|LoadLevel))

(event EventBeginPlay
  ;[1 1 1] Load the first level
  (CallFunction|LoadNextLevel))

(fn ConstructionScript)

(fn SpawnObjects
  (bind _currentlocation (LocalVariables|GetCurrentLocation))
  (bind _currenttilemap (Variables|Default|GetCurrentTilemap))
  (bind _mapheight (Variables|/Script/Paper2D.PaperTileMap|GetMapHeight _currenttilemap))
  (bind _mapwidth (Variables|/Script/Paper2D.PaperTileMap|GetMapWidth _currenttilemap))
  (LocalVariables|SetHeight (- _mapheight 1))
  (LocalVariables|SetWidth (- _mapwidth 1))
  (for _index (range 0 (* _mapwidth _mapheight))
    _)
  (for (_ _array_index) (Variables|/Script/Paper2D.PaperTileMap|GetTileLayers _currenttilemap)
    (for _index_2 (range 0 (LocalVariables|GetWidth))
      (Utilities|Array|SetArrayElem _currentlocation _index_2 0)
      (for _index_3 (range 0 (LocalVariables|GetHeight))
        (Utilities|Array|SetArrayElem _currentlocation 1 _index_3)
        (LocalVariables|SetSpawnLocation (Math|Transform|MakeTransform (Math|Vector|MakeVector (* 1e+02 _index_2) (* 1e+02 _index_3) 0.0) "0, 0, 0" "1.000000,1.000000,1.000000"))
        (Utilities|FlowControl|Sequence
          (:then_0
            (switch string (Utilities|String|ToString(Name) (Class|TileMapBlueprintLibrary|GetTileUserData (Class|PaperTileMapComponent|GetTile (Variables|Default|GetLevel%20Tilemap) _index_2 _index_3 _array_index)))
              (:PlayerSpawn
                ;[1 1 1] Spawn player
                (bind _returnvalue (Game|SpawnActorfromClass "/Game/Blueprints/DieWorld/BP_TestPawn.BP_TestPawn_C" (LocalVariables|GetSpawnLocation) "Undefined" 0 0))
                (Pawn|Possess (Game|GetPlayerController 0) _returnvalue)
                (Variables|/Game/Blueprints/DieWorld/BP_TestPawn.BP_TestPawn_C|SetLevelManager _returnvalue self)
                (Utilities|Array|Add (Variables|Default|GetGridItems) _returnvalue))
              (:Key
                ;[1 1 1] Spawn Key
                (bind _returnvalue_2 (Game|SpawnActorfromClass "/Game/Blueprints/Objects/BP_Key.BP_Key_C" (LocalVariables|GetSpawnLocation) "Undefined" 0 0))
                (Utilities|Array|Add (Variables|Default|GetGridItems) _returnvalue_2))
              (:Hazard
                ;[1 1 1] Spawn hazard
                (bind _returnvalue_3 (Game|SpawnActorfromClass "/Game/Blueprints/Objects/BP_Hazard.BP_Hazard_C" (LocalVariables|GetSpawnLocation) "Undefined" 0 0))
                (Utilities|Array|Add (Variables|Default|GetGridItems) _returnvalue_3))
              (:EnemySpawnLeft
                ;[1 1 1] Spawn enemy
                (LocalVariables|SetEnemyDirection "NewEnumerator1")
                (bind _returnvalue_4 (Game|SpawnActorfromClass "/Game/Blueprints/Objects/BP_Enemy.BP_Enemy_C" (LocalVariables|GetSpawnLocation) "Undefined" 0 0 :!label _label))
                (Variables|/Game/Blueprints/Objects/BP_Enemy.BP_Enemy_C|SetGridX _returnvalue_4 (Math|Float|Truncate (/ (.x (Math|Transform|TransformLocation (LocalVariables|GetSpawnLocation) "0, 0, 0")) 1e+02)))
                (Variables|/Game/Blueprints/Objects/BP_Enemy.BP_Enemy_C|SetGridY _returnvalue_4 (Math|Float|Truncate (/ (.y (Math|Transform|TransformLocation (LocalVariables|GetSpawnLocation) "0, 0, 0")) 0.0)))
                (Default|ChangeDirection _returnvalue_4 (LocalVariables|GetEnemyDirection))
                (Variables|/Game/Blueprints/Objects/BP_Enemy.BP_Enemy_C|SetLevelManager _returnvalue_4 self)
                (Utilities|Array|Add (Variables|Default|GetGridItems) _returnvalue_4))
              (:EnemySpawnRight
                (LocalVariables|SetEnemyDirection "NewEnumerator3")
                (goto _label))
              (:EnemySpawnUp
                (LocalVariables|SetEnemyDirection "NewEnumerator0")
                (goto _label))
              (:EnemySpawnDown
                (LocalVariables|SetEnemyDirection "NewEnumerator2")
                (goto _label))
              (:Exit
                ;[1 1 1] Spawn exit
                (bind _returnvalue_5 (Game|SpawnActorfromClass "/Game/Blueprints/BP_LevelTransition.BP_LevelTransition_C" (LocalVariables|GetSpawnLocation) "Undefined" 0 0))
                (Utilities|Array|Add (Variables|Default|GetGridItems) _returnvalue_5))))
          (:then_1
            (if (and (LocalVariables|GetDrawTiles) (not (Utilities|Enum|Equal(Enum) (Utilities|String|ToString(Name) (Class|TileMapBlueprintLibrary|GetTileUserData (Class|PaperTileMapComponent|GetTile (Variables|Default|GetLevel%20Tilemap) _index_2 _index_3 _array_index))) "Block")))
              ;[1 1 1] Spawn tiles
              (bind _returnvalue_6 (Game|SpawnActorfromClass "/Game/Blueprints/Objects/BP_TileIndicator.BP_TileIndicator_C" (LocalVariables|GetSpawnLocation) "Undefined" 0 0))
              (if (LocalVariables|GetEvenTile)
                (Default|SetMaterial _returnvalue_6 "/Game/Blueprints/Objects/M_Tile1.M_Tile1")
                (else
                  (Default|SetMaterial _returnvalue_6 "/Game/Blueprints/Objects/M_Tile2.M_Tile2")))
              (Utilities|Array|Add (Variables|Default|GetGridTiles) _returnvalue_6)))
          (:then_2
            (LocalVariables|SetEvenTile (not (LocalVariables|GetEvenTile)))))))
    (LocalVariables|SetDrawTiles (not (LocalVariables|GetDrawTiles))))
  (Development|PrintString "Hello"))

(fn GetArrayIndex
  (params (x :type Integer) (y :type Integer) (width :type Integer))
  (return (+ (* x width) y)))

(fn LoadLevel
  (bind _returnvalue (Utilities|GetDataTableRow "/Game/Levels/Tilemaps/DT_LevelBudgets.DT_LevelBudgets" (Utilities|String|StringToName (Utilities|String|ToString(Integer) (Variables|Default|GetCurrentLevel))))
    (:then
      (Class|PaperTileMapComponent|SetTileMap (Variables|Default|GetLevel%20Tilemap) (.AssociatedTilemap (Utilities|Struct|BreakSTRUCT_LevelBudget _returnvalue)))
      (Variables|Default|SetCurrentTilemap (.AssociatedTilemap (Utilities|Struct|BreakSTRUCT_LevelBudget _returnvalue)))
      (LevelLoading|SpawnObjects))))

(fn UnloadLevel
  (LevelUnloading|ClearActors (Variables|Default|GetGridItems))
  (LevelUnloading|ClearActors (Variables|Default|GetGridTiles)))

(fn ClearActors
  (params (ActorsToClear :type Array%20of%20Actor%20Object%20References))
  (for _array_element ActorsToClear
    (Utilities|IsValid _array_element
      (:Is%20Valid
        (Actor|DestroyActor _array_element))))
  (Utilities|Array|Clear ActorsToClear))