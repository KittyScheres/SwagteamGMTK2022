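; BP_Hazard is a one-shot hazard that costs the player pawn steps on contact and rearms when the player resets.
; Overlapping Box1 while active calls SubstractSteps on BP_TestPawn and clears IsActive.
; On BeginPlay it registers a reset event through the pawn's AssignPlayerReset, which sets IsActive again.
; Tick mirrors IsActive to actor visibility and feeds the player camera manager to the Bilboarding target.
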(event OnComponentBeginOverlap(Box1)
  (params (OverlappedComponent :type Primitive%20Component%20Object%20Reference) (OtherActor :type Actor%20Object%20Reference) (OtherComp :type Primitive%20Component%20Object%20Reference) (OtherBodyIndex :type Integer) (bFromSweep :type Boolean) (SweepResult :type Hit%20Result%20Structure%20%28by%20ref%29))
  (if (Variables|Default|GetIsActive)
    (bind _asbp_test_pawn (Utilities|Casting|CastToBP_TestPawn OtherActor))
    (Default|SubstractSteps _asbp_test_pawn 2)
    (Variables|Default|SetIsActive false)))

(event Custom|PlayerReset_Event_0
  (Variables|Default|SetIsActive true))

(event EventBeginPlay
  (bind _returnvalue (Actor|GetActorOfClass "/Game/Blueprints/DieWorld/BP_TestPawn.BP_TestPawn_C"))
  (bind _output_get (Variables|Default|SetPlayerRef _returnvalue))
  (EventDispatchers|AssignPlayerReset _output_get (delegate Custom|PlayerReset_Event_0)))

(event Collision|EventActorBeginOverlap
  (params (OtherActor :type Actor%20Object%20Reference)))

(event EventTick
  (params (DeltaSeconds :type Float%20%28single-precision%29))
  (Variables|/Game/Blueprints/Component/Bilboarding.Bilboarding_C|SetTargetLocation (Variables|Default|GetBilboarding) (Game|GetPlayerCameraManager 0))
  (if (Variables|Default|GetIsActive)
    (Rendering|SetActorHiddenInGame false)
    (else
      (Rendering|SetActorHiddenInGame true))))

(fn ConstructionScript)