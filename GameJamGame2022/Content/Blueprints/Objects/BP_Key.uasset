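; Collectible key pickup that increments the key count on BP_TestPawn when that pawn overlaps its box.
; Collection clears IsActive; Tick hides the actor while inactive, prints the pawn's key count, and feeds the camera manager to a billboarding target.
; BeginPlay binds to the pawn's player reset event, which reactivates the key so it can be collected again.
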(event OnComponentBeginOverlap(Box)
  (params (OverlappedComponent :type Primitive%20Component%20Object%20Reference) (OtherActor :type Actor%20Object%20Reference) (OtherComp :type Primitive%20Component%20Object%20Reference) (OtherBodyIndex :type Integer) (bFromSweep :type Boolean) (SweepResult :type Hit%20Result%20Structure%20%28by%20ref%29))
  (if (Variables|Default|GetIsActive)
    (bind _asbp_test_pawn (Utilities|Casting|CastToBP_TestPawn OtherActor))
    (Variables|/Game/Blueprints/DieWorld/BP_TestPawn.BP_TestPawn_C|SetAmountOfKeysCollected _asbp_test_pawn (+ (Variables|/Game/Blueprints/DieWorld/BP_TestPawn.BP_TestPawn_C|GetAmountOfKeysCollected _asbp_test_pawn) 1))
    (Variables|Default|SetIsActive false)))

(event Custom|PlayerResetEvent
  (Variables|Default|SetIsActive true))

(event EventBeginPlay
  (bind _returnvalue (Actor|GetActorOfClass "/Game/Blueprints/DieWorld/BP_TestPawn.BP_TestPawn_C"))
  (bind _output_get (Variables|Default|SetPlayerref _returnvalue))
  (EventDispatchers|BindEventtoPlayerReset _output_get (delegate Custom|PlayerResetEvent)))

(event EventTick
  (params (DeltaSeconds :type Float%20%28single-precision%29))
  (Variables|/Game/Blueprints/Component/Bilboarding.Bilboarding_C|SetTargetLocation (Variables|Default|GetBilboarding) (Game|GetPlayerCameraManager 0))
  (if (Variables|Default|GetIsActive)
    (Rendering|SetActorHiddenInGame false)
    (else
      (Rendering|SetActorHiddenInGame true)
      (Development|PrintString (Utilities|String|ToString(Integer) (Variables|/Game/Blueprints/DieWorld/BP_TestPawn.BP_TestPawn_C|GetAmountOfKeysCollected (Variables|Default|GetPlayerref))) true true "(R=1.000000,G=0.000000,B=0.000000,A=1.000000)"))))

(fn ConstructionScript)