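; Level transition trigger that rotates the BP_DieDefinition actor 90 degrees in pitch, apparently a hardcoded test.
; BeginPlay finds the die and caches its six cube components.
; The first BP_TestPawn overlap with the trigger Cube shows all six and stores start and goal rotations.
; Tick lerps between them by a fixed, frame-rate-dependent step, printing the alpha, then hides Cube3 when done.
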(event OnComponentBeginOverlap(Cube)
  (params (OverlappedComponent :type Primitive%20Component%20Object%20Reference) (OtherActor :type Actor%20Object%20Reference) (OtherComp :type Primitive%20Component%20Object%20Reference) (OtherBodyIndex :type Integer) (bFromSweep :type Boolean) (SweepResult :type Hit%20Result%20Structure%20%28by%20ref%29))
  (bind _worldref (Variables|Default|GetWorldref))
  (bind _returnvalue (Transformation|GetActorRotation _worldref))
  ;[1 1 1] Hardcoded test rotation
  (Utilities|Casting|CastToBP_TestPawn OtherActor)
  (Utilities|FlowControl|DoOnce false
    (:Completed
      (for _array_element (Variables|Default|GetAllCubes)
        (Rendering|SetVisibility _array_element true false))
      (Variables|Default|SetOngoingTransition true)
      (Variables|Default|SetRotateOrigin (Transformation|GetActorRotation (Variables|Default|GetWorldref)))
      (Variables|Default|SetRotateGoal (Math|Rotator|MakeRotator (.roll _returnvalue) (+ (.pitch _returnvalue) 9e+01) (.yaw _returnvalue))))))

(event EventBeginPlay
  (bind _returnvalue (Actor|GetActorOfClass "/Game/Blueprints/DieWorld/BP_DieDefinition.BP_DieDefinition_C"))
  (Variables|Default|SetWorldref _returnvalue)
  (Variables|Default|SetAllCubes (Utilities|Array|MakeArray (Variables|/Game/Blueprints/DieWorld/BP_DieDefinition.BP_DieDefinition_C|GetCube (Variables|Default|GetWorldref)) (Variables|/Game/Blueprints/DieWorld/BP_DieDefinition.BP_DieDefinition_C|GetCube1 (Variables|Default|GetWorldref)) (Variables|/Game/Blueprints/DieWorld/BP_DieDefinition.BP_DieDefinition_C|GetCube2 (Variables|Default|GetWorldref)) (Variables|/Game/Blueprints/DieWorld/BP_DieDefinition.BP_DieDefinition_C|GetCube3 (Variables|Default|GetWorldref)) (Variables|/Game/Blueprints/DieWorld/BP_DieDefinition.BP_DieDefinition_C|GetCube4 (Variables|Default|GetWorldref)) (Variables|/Game/Blueprints/DieWorld/BP_DieDefinition.BP_DieDefinition_C|GetCube5 (Variables|Default|GetWorldref)))))

(event Collision|EventActorBeginOverlap
  (params (OtherActor :type Actor%20Object%20Reference)))

(event EventTick
  (params (DeltaSeconds :type Float%20%28single-precision%29))
  (if (Variables|Default|GetOngoingTransition)
    (bind _output_get (Variables|Default|SetInterpolater (+ (Variables|Default|GetInterpolater) 0.01)))
    (Development|PrintString (Utilities|String|ToString(Float) _output_get))
    (Transformation|SetActorRotation (Variables|Default|GetWorldref) (Math|Rotator|Lerp(Rotator) (Variables|Default|GetRotateOrigin) (Variables|Default|GetRotateGoal) (Math|Float|Clamp(Float) (Variables|Default|GetInterpolater))))
    (if (> (Variables|Default|GetInterpolater) 1.0)
      (Rendering|SetVisibility (Variables|/Game/Blueprints/DieWorld/BP_DieDefinition.BP_DieDefinition_C|GetCube3 (Variables|Default|GetWorldref)) false false)
      (Variables|Default|SetOngoingTransition false))))

(fn ConstructionScript)